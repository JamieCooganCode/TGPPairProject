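; Breakable pot actor that drops a stamina pickup when a player weapon overlaps it.
; The overlap damages its Destructible component, spawns a pickup at the pot collider, then destroys the actor after a short delay.
; A random roll chooses big or small pickup, but its range excludes the tested zero, so only the small one spawns.
; No guard blocks repeat overlaps during the delay.
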(event `self.ReceiveActorBeginOverlap`
  (params (OtherActor :type "Actor Object Reference"))
  (bind _returnvalue (`SceneComponent.K2_GetComponentToWorld` (`self.PotCollider`)))
  (cast `BasePlayerWeapon` OtherActor)
  (`DestructibleComponent.ApplyDamage` (`self.Destructible`) 10.0 (`SceneComponent.K2_GetComponentLocation` (`self.Destructible`)) (0.0 0.0 1.0) 10.0)
  (if (== (`KismetMathLibrary.RandomIntegerInRange` 1 4) 0)
    (`|SpawnActorFromClass` "/Game/Blueprints/Pickup_BPs/MyBPStaminaBIgPickup.MyBPStaminaBIgPickup_C" _returnvalue "Undefined" "OverrideRootScale" null null)
    (else
      (`|SpawnActorFromClass` "/Game/Blueprints/Pickup_BPs/MyBPStaminSmallPickup.MyBPStaminSmallPickup_C" _returnvalue "Undefined" "OverrideRootScale" null null)))
  (`KismetSystemLibrary.Delay` 5.0)
  (`self.K2_DestroyActor` self))

(fn `UserConstructionScript`)
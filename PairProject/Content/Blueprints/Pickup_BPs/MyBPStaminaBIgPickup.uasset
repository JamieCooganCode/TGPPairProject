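; Large stamina pickup Blueprint that restores stamina to a BaseCharacter that overlaps it.
; On BeginPlay it moves the pickup model to the collider's world location.
; On overlap it casts the other actor to BaseCharacter, increases its current stamina by a fixed amount, prints the new value and calls AfterPickedUp.
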(event `self.ReceiveBeginPlay`
  (`SceneComponent.K2_SetWorldLocation` (`self.pickupModel`) (`SceneComponent.K2_GetComponentLocation` (`self.pickupCollider`)) false false))

(event `self.ReceiveActorBeginOverlap`
  (params (OtherActor :type "Actor Object Reference"))
  (bind _asbase_character (cast `BaseCharacter` OtherActor))
  (`BaseCharacter.IncreaseCurrentStamina` _asbase_character 10.0)
  (`KismetSystemLibrary.PrintString` (`KismetStringLibrary.Conv_DoubleToString` (`BaseCharacter.CurrentStamina` _asbase_character)))
  (`self.AfterPickedUp`))

(fn `UserConstructionScript`)
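; Biggoron Knife melee weapon Blueprint that registers sword hits on enemies.
; On BeginPlay it moves SwordMesh to the world location of AttackCollider.
; Any actor overlap gathers all currently overlapping BaseEnemy, BomberEnemy and FreezeEnemy actors with separate class queries and passes each list to OnBeginSwordOverlap.
; Hit handling is not defined in this graph, and Tick and the construction script are empty.
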(event `self.ReceiveBeginPlay`
  (`SceneComponent.K2_SetWorldLocation` (`self.SwordMesh`) (`SceneComponent.K2_GetComponentLocation` (`self.AttackCollider`)) false false))

(event `self.ReceiveActorBeginOverlap`
  (params (OtherActor :type "Actor Object Reference"))
  (`self.OnBeginSwordOverlap` (`self.GetOverlappingActors` "/Script/PairProject.BaseEnemy"))
  (`self.OnBeginSwordOverlap` (`self.GetOverlappingActors` "/Script/PairProject.BomberEnemy"))
  (`self.OnBeginSwordOverlap` (`self.GetOverlappingActors` "/Script/PairProject.FreezeEnemy")))

(fn `UserConstructionScript`)
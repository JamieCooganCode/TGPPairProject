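; Playable Impa character Blueprint that sets up its camera, carries a Biggoron Knife and opens pause and map screens.
; BeginPlay positions and configures the spring-arm camera, then spawns the knife and attaches its mesh and attack collider to the left-hand socket.
; Tick applies yaw input and polls button flags to pause with a menu or show Impa's map overlay.
; Otherwise, while moving, it snaps facing to the movement direction, throttled by a DoOnce and delay.
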(event `self.ReceiveBeginPlay`
  (bind _mesh (`self.Mesh`))
  (`SceneComponent.K2_SetWorldLocation` (`self.CameraSpringArm`) (- (`SceneComponent.K2_GetComponentLocation` (`self.CapsuleComponent`)) (150.0 0.0 -300.0)) false false)
  (`self.SetUpCameraArm` self)
  (`self.SetUpCamera` self)
  (bind _returnvalue (`|SpawnActorFromClass` "/Game/Blueprints/Weapon_BPs/MyBiggoronKnifeWeapon.MyBiggoronKnifeWeapon_C" (`SceneComponent.K2_GetComponentToWorld` _mesh) "Undefined" "OverrideRootScale" null null))
  (`SceneComponent.K2_AttachToComponent` (`BasePlayerWeapon.SwordMesh` _returnvalue) _mesh "LeftHandSocket" "SnapToTarget" "SnapToTarget" "KeepRelative" true)
  (`SceneComponent.K2_AttachToComponent` (`BasePlayerWeapon.AttackCollider` _returnvalue) _mesh "LeftHandSocket" "SnapToTarget" "SnapToTarget" "KeepRelative" true))

(event `self.ReceiveTick`
  (params (DeltaSeconds :type "Float (single-precision)"))
  (`self.AddControllerYawInput` self (`self.CurrentRotation`))
  (if (`self.StartButtonHit`)
    (`GameplayStatics.SetGamePaused` true)
    (bind _returnvalue (`|CreateWidget` "/Game/UIs/Pause_Menu.Pause_Menu_C"))
    (`UserWidget.AddToViewport` _returnvalue 0)
    (elif (`self.BackButtonHit`)
      (bind _returnvalue_2 (`|CreateWidget` "/Game/UIs/ImpaMap_Overlay.ImpaMap_Overlay_C"))
      (`UserWidget.AddToViewport` _returnvalue_2 0)
      (elif (`self.movingToPosition`)
        (`/Engine/EditorBlueprintResources/StandardMacros.DoOnce` false :!label _label
          (:`Completed`
            (`self.Rotate To Keep`)
            (`KismetSystemLibrary.Delay` 1.0)
            (goto _label :!via `Reset`)))))))

(event `Rotate To Keep`
  (`self.K2_SetActorRotation` (`KismetMathLibrary.Conv_VectorToRotator` (`self.DirectionToGo`))))

(fn `UserConstructionScript`)
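; Player character Blueprint, named for Link, with a spring-arm camera, an equipped sword and pause handling.
; BeginPlay offsets the spring arm from the capsule, runs camera setup, then spawns the weapon and attaches its sword mesh and attack collider to the right-hand socket.
; Tick feeds CurrentRotation into controller yaw and, when StartButtonHit is set, pauses the game and shows a new pause menu.
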(event `self.ReceiveBeginPlay`
  (bind _mesh (`self.Mesh`))
  (`SceneComponent.K2_SetWorldLocation` (`self.CameraSpringArm`) (- (`SceneComponent.K2_GetComponentLocation` (`self.CapsuleComponent`)) (150.0 0.0 -300.0)) false false)
  (`self.SetUpCameraArm` self)
  (`self.SetUpCamera` self)
  (bind _returnvalue (`|SpawnActorFromClass` "/Game/Blueprints/Weapon_BPs/MyBPBasePlayerWeapon.MyBPBasePlayerWeapon_C" (`SceneComponent.K2_GetComponentToWorld` _mesh) "Undefined" "OverrideRootScale" null null))
  (`SceneComponent.K2_AttachToComponent` (`BasePlayerWeapon.SwordMesh` _returnvalue) _mesh "RightHandSocket" "SnapToTarget" "SnapToTarget" "KeepRelative" true)
  (`SceneComponent.K2_AttachToComponent` (`BasePlayerWeapon.AttackCollider` _returnvalue) _mesh "RightHandSocket" "SnapToTarget" "SnapToTarget" "KeepRelative" true))

(event `self.ReceiveTick`
  (params (DeltaSeconds :type "Float (single-precision)"))
  (`self.PlayerRotate`)
  (if (`self.StartButtonHit`)
    (`GameplayStatics.SetGamePaused` true)
    (bind _returnvalue (`|CreateWidget` "/Game/UIs/Pause_Menu.Pause_Menu_C"))
    (`UserWidget.AddToViewport` _returnvalue 0)))

(fn `PlayerRotate`
  (`self.AddControllerYawInput` self (`self.CurrentRotation`)))

(fn `UserConstructionScript`)